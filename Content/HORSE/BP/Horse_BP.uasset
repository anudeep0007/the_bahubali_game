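; Horse_BP is a rideable horse character driven by player movement, look, sprint and jump input.
; Movement follows the control rotation while grounded, updating Speed and Direction, with Shift overriding Speed for sprinting.
; Space triggers a timed jump only while moving forward.
; E dismounts by possessing the stored third-person rider, playing a dismount animation, then restoring its collision, mount-point location and Animation Blueprint mode.
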(event `InputAxis|MoveForward`
  (params (AxisValue :type "Float (single-precision)"))
  (bind _returnvalue (`self.GetControlRotation`))
  (if (not (`NavMovementComponent.IsFalling` (`self.CharacterMovement`)))
    (bind _output_get (set `self.speed` (* AxisValue 2.0)))
    (bind _output_get_2 (set `self.Direction` (.yaw (`KismetMathLibrary.NormalizedDeltaRotator` (`self.K2_GetActorRotation`) _returnvalue))))
    (`KismetSystemLibrary.PrintString` (`KismetStringLibrary.Conv_DoubleToString` _output_get_2))
    (`self.AddMovementInput` (`KismetMathLibrary.GetForwardVector` _returnvalue) _output_get)
    (if (`self.sprint`)
      (set `self.speed` 5.0)
      (else
        (set `self.speed` (`self.speed`))))))

(event `InputAxis|LookUp`
  (params (AxisValue :type "Float (single-precision)"))
  (`self.AddControllerPitchInput` AxisValue))

(event `InputAxis|LookSide`
  (params (AxisValue :type "Float (single-precision)"))
  (`self.AddControllerYawInput` AxisValue))

(event `self.ReceiveTick`
  (params (DeltaSeconds :type "Float (single-precision)")))

(event `self.ReceiveBeginPlay`)

(event `Key|LeftShift`
  (params (Key :type "Key Structure"))
  (:`Pressed`
    (set `self.sprint` true))
  (:`Released`
    (set `self.sprint` false)))

(event `Key|SpaceBar`
  (params (Key :type "Key Structure"))
  (:`Pressed`
    (if (> (`self.speed`) 0.1)
      (`self.Jump`)
      (set `self.can jump` true)
      (`KismetSystemLibrary.Delay` 0.5)
      (set `self.can jump` false)
      (`self.StopJumping`))))

(event `Key|E`
  (params (Key :type "Key Structure"))
  (bind _thirdperson (`self.thirdperson`))
  (bind _mesh (`Character.Mesh` _thirdperson))
  (:`Pressed`
    (`Controller.Possess` (`GameplayStatics.GetPlayerController` 0) _thirdperson)
    (`SkeletalMeshComponent.PlayAnimation` _mesh "/Game/HorseAnimsetPro/Animations/Rider_Mannequin_V2/Rider_Dismount_Front_Right_v2.Rider_Dismount_Front_Right_v2" false)
    (`KismetSystemLibrary.Delay` 1.16)
    (`PrimitiveComponent.SetCollisionEnabled` (`Character.CapsuleComponent` (`self.thirdperson`)) "QueryAndPhysics")
    (`self.K2_SetActorLocation` _thirdperson (`SceneComponent.K2_GetComponentLocation` (`self.mount point`)) false false)
    (`SkeletalMeshComponent.SetAnimationMode` _mesh "AnimationBlueprint")))

(fn `UserConstructionScript`)